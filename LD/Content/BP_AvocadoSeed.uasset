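; BP_AvocadoSeed is an avocado seed actor that can be thrown as a physics object.
; ThwowSeed enables physics and collision on its Sphere, then applies an impulse built from the normalized forward vector scaled by ThrowForce, plus the passed Location.
; It also draws a long-lived debug arrow from Location to that same vector.
; RecoverSeed is an empty stub, and an AddImpulseAtLocation variant is left unconnected.
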(event Custom|ThwowSeed
  (params (ForwardVec :type Vector) (Location :type Vector))
  (bind _returnvalue (Math|Vector|Normalize ForwardVec))
  (bind _sphere (Variables|Default|GetSphere))
  (bind _throwforce (Variables|Default|GetThrowForce))
  (bind _returnvalue_2 (* _returnvalue _throwforce))
  (bind _returnvalue_3 (+ _returnvalue_2 Location))
  (Physics|SetSimulatePhysics _sphere true)
  (Collision|SetCollisionEnabled _sphere "QueryAndPhysics")
  (Physics|AddImpulse (Variables|Default|GetSphere) _returnvalue_3 "None" false)
  (Rendering|Debug|DrawDebugArrow Location _returnvalue_3 1e+02 "(R=0.278669,G=0.770833,B=0.494483,A=1.000000)" 3e+01 2.0))

(event Custom|RecoverSeed)

(event EventBeginPlay)

(event Collision|EventActorBeginOverlap
  (params (OtherActor :type Actor%20Object%20Reference)))

(event EventTick
  (params (DeltaSeconds :type Float%20%28single-precision%29)))

(fn ConstructionScript)